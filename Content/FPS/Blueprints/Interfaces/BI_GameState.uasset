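; BI_GameState is a Blueprint interface, named for the game state, that declares match-level calls for the FPS game.
; It covers team changes, player death handling, player spawning, bot respawning, and messages to everyone or per team with a reliability flag.
; Query functions expose game mode widgets, match objectives, the game mode enum, a menu check and the AI behavior tree.
; It contains only signatures with no logic, leaving behavior to implementers.
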(fn `GetAIBehaivorTree`
  (returns (BehaviorTree :type "BehaviorTree Object Reference"))
  (return null))

(fn `GetGameMode`
  (returns (GM :type "/Game/FPS/Maps/Enums/EGameModes Enum"))
  (return "NewEnumerator4"))

(fn `GetGameModeWidgets`
  (returns (GameModeWidget :type "UserWidget Soft Class Reference") (ScoresBoard :type "UserWidget Soft Class Reference") (EndGameSocores :type "UserWidget Soft Class Reference"))
  (return null null null))

(fn `GetMatchObjectives`
  (returns (Objectives :type "Array of Actor Object Reference"))
  (return))

(fn `HandlePlayerDead`
  (params (Team :type Integer) (DeadActor :type "Actor Object Reference") (Instigator :type "Controller Object Reference"))
  (return))

(fn `IsMenu`
  (returns (IsMenu :type Boolean))
  (return false))

(fn `OnTeamChanged`)

(fn `RespawnBot`
  (params (BotController :type "Controller Object Reference")))

(fn `SendMessageTeam`
  (params (MessageTeam0 :type Text) (MessageTeam1 :type Text) (Reliable :type Boolean)))

(fn `SendMessageToAll`
  (params (Message :type Text) (Reliable :type Boolean)))

(fn `SpawnPlayer`
  (params (PlayerController :type "PlayerController Object Reference")))