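; Claymore lethal equipment that, on release, asks the server to place an explosive on the surface just in front of its owner.
; The server traces down for a surface, then checks that the path from the owner to that spot is clear.
; Valid spots spawn ExplosiveToSpawn aligned to control yaw with an offset and reduce AC_InventorySystem lethal ammo.
; Failed traces trigger a client event showing a not-enough-space error widget.
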(event `self.OnRelease`
  ;[0 0 0] On Release
  (`self.Server_TryToSpawnClaymore`))

(event `Server_TryToSpawnClaymore`
  (bind _returnvalue (`self.GetOwner`))
  (bind _returnvalue_2 (`self.GetOwner`))
  (bind _returnvalue_3 (`self.GetComponentByClass` (`self.GetOwner`) "/Game/FPS/Blueprints/BlueprintsComponents/AC_InventorySystem.AC_InventorySystem_C"))
  (bind (_returnvalue_roll _returnvalue_pitch _returnvalue_yaw) (`KismetMathLibrary.BreakRotator` (`Controller.GetControlRotation` (`self.GetInstigatorController` _returnvalue_2))))
  (bind _returnvalue_4 (+ (`self.K2_GetActorLocation` _returnvalue) (* (`self.GetActorForwardVector` _returnvalue) 100.0)))
  ;[0 0 0 0.5] Try to spawn
  (bind _outhit (`KismetSystemLibrary.LineTraceSingle` _returnvalue_4 (+ _returnvalue_4 (* (`self.GetActorUpVector` _returnvalue) -200.0)) "TraceTypeQuery1" false (`|MakeArray` self :!type "Actor Object Reference")))
  (if (`GameplayStatics.BreakHitResult` _outhit)
    (bind _outhit_2 (`KismetSystemLibrary.LineTraceSingle` (`self.K2_GetActorLocation` (`self.GetOwner`)) (+ (`.Location` (`GameplayStatics.BreakHitResult` _outhit)) (0.0 0.0 10.0)) "TraceTypeQuery1" false (`|MakeArray` (`self.GetOwner`))))
    (if (`GameplayStatics.BreakHitResult` _outhit_2)
      (`self.Client_ShowFailMessage`)
      (else
        ;[0 0 0] Spawn
        (bind _returnvalue_5 (`|SpawnActorFromClass` (`self.ExplosiveToSpawn`) (`KismetMathLibrary.MakeTransform` (`.Location` (`GameplayStatics.BreakHitResult` _outhit)) (`KismetMathLibrary.MakeRotator` 0.0 0.0 (- _returnvalue_yaw 90.0))) "Undefined" "SelectDefaultAtRuntime" _returnvalue_2 (cast `Pawn` _returnvalue_2 :!pure true)))
        (`/Engine/EditorBlueprintResources/StandardMacros.IsValid` _returnvalue_5
          (:`Is Valid`
            (`/Engine/EditorBlueprintResources/StandardMacros.IsValid` _returnvalue_3
              (:`Is Valid`
                (`/Game/FPS/Blueprints/BlueprintsComponents/AC_InventorySystem.ReduceLethalAmmo` _returnvalue_3)))))))
    (else
      (`self.Client_ShowFailMessage`))))

(event `Client_ShowFailMessage`
  ;[0 0 0 0.5] Fail Message
  (bind _returnvalue (`|CreateWidget` "/Game/FPS/UI/Gameplay/WB_Error_Message.WB_Error_Message_C" (`GameplayStatics.GetPlayerController` 0) "Not Enought Space"))
  (`UserWidget.AddToViewport` _returnvalue 0))

(fn `UserConstructionScript`
  (`parent.UserConstructionScript`)
  (set `self.UI_Icon` "/Game/FPS/UI/Textures/T_Claymore.T_Claymore"))