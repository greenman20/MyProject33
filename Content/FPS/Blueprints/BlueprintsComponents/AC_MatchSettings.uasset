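; AC_MatchSettings is an actor component that stores match configuration for the FPS game.
; It exposes getters and setters for bot counts per team, AI difficulty, friendly fire, player cap, score targets and time limits.
; Some values, such as respawn, rounds to win and game mode, have getters only, and bot difficulty has two setters writing the same variable.
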(fn `Get Match With Time Limit`
  (returns (MatchWithTimeLimit :type Boolean))
  (return (`self.bMatchWithTimeLimit`)))

(fn `GetAIDifficulty`
  (returns (BotDifficulty :type "/Game/FPS/AI/E_AI_Difficulty Enum"))
  (return (`self.AIDifficulty`)))

(fn `GetAllowBots`
  (returns (bAllowBots :type Boolean))
  (return (`self.bAllowBots`)))

(fn `GetAllowFriendlyFire`
  (returns (bAllowFriendlyFire :type Boolean))
  (return (`self.bAllowFriendlyFire`)))

(fn `GetAllowRespawn`
  (returns (bAllowRespawn :type Boolean))
  (return (`self.bAllowRespawn`)))

(fn `GetGameMode`
  (returns (GameMode :type "/Game/FPS/Maps/Enums/EGameModes Enum"))
  (return (`self.GameMode`)))

(fn `GetGameModeName`
  (returns (GameMode :type "/Game/FPS/Blueprints/Enums/E_GameModeNames Enum"))
  (return (`self.GameModeName`)))

(fn `GetMaxPlayers`
  (returns (MaxPlayers :type Integer))
  (return (`self.MaxPlayers`)))

(fn `GetPointsToWin`
  (returns (PointsToWin :type Integer))
  (return (`self.PointsToWin`)))

(fn `GetRoundsToWin`
  (returns (RoundsToWin :type Integer))
  (return (`self.RoundsToWin`)))

(fn `GetTeamABots`
  (returns (BotsTeamA :type Integer))
  (return (`self.BotsTeamA`)))

(fn `GetTeamBBots`
  (returns (BotsTeamB :type Integer))
  (return (`self.BotsTeamB`)))

(fn `SetAIDifficulty`
  (params (AIDifficulty :type "/Game/FPS/AI/E_AI_Difficulty Enum" :default "NewEnumerator0"))
  (set `self.AIDifficulty` AIDifficulty))

(fn `SetAllowBots`
  (params (bAllowBots :type Boolean))
  (set `self.bAllowBots` bAllowBots))

(fn `SetAllowFriendlyFire`
  (params (bAllowFriendlyFire :type Boolean))
  (set `self.bAllowFriendlyFire` bAllowFriendlyFire))

(fn `SetBotDifficulty`
  (params (BotDifficulty :type "/Game/FPS/AI/E_AI_Difficulty Enum" :default "NewEnumerator0"))
  (set `self.AIDifficulty` BotDifficulty))

(fn `SetBotsTeamA`
  (params (BotsTeamA :type Integer))
  (set `self.BotsTeamA` BotsTeamA))

(fn `SetBotsTeamB`
  (params (BotsTeamB :type Integer))
  (set `self.BotsTeamB` BotsTeamB))

(fn `SetMaxPlayers`
  (params (MaxPlayers :type Integer))
  (set `self.MaxPlayers` MaxPlayers))

(fn `SetPointsToWin`
  (params (PointsToWin :type Integer))
  (set `self.PointsToWin` PointsToWin))

(fn `SetRoundTimeLimit`
  (params (RoundTimeLimit :type "Float (double-precision)"))
  (set `self.RoundTimeLimit` RoundTimeLimit))