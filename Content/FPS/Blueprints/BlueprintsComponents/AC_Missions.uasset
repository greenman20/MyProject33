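; Mission component that tracks the player's kill and win missions in the FPS and awards XP through its owner.
; On BeginPlay it loads missions from a save slot, creating three data-asset defaults if no save exists.
; PlayerKilled and the authority-only winner binding, which checks player 0's team, advance missions filtered by weapon or game mode.
; Progress saves asynchronously; unlike kill checks, win checks do not skip completed missions and save before marking completion.
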(event `self.ReceiveBeginPlay`
  ;[0 0 0] BeginPlay
  (`self.LoadMissions`)
  (`/Engine/EditorBlueprintResources/ActorComponentMacros.Switch Has Authority`
    (:`Authority`
      (add `/Game/FPS/Blueprints/BlueprintsComponents/AC_MatchStateSystem.WinnerTeamSelected` (`Actor.GetComponentByClass` (`GameplayStatics.GetGameState`) "/Game/FPS/Blueprints/BlueprintsComponents/AC_MatchStateSystem.AC_MatchStateSystem_C") (delegate `OnWinnerTeamSelected`)))))

(event `OnWinnerTeamSelected`
  (params (WinnerTeam :type Integer))
  ;[0 0 0] BeginPlay
  ;;[0 0 0] On WinnerTeamSelected
  (bind _team (message `/Game/FPS/Blueprints/Interfaces/BI_PlayerState.GetTeam` (`Pawn.PlayerState` (`GameplayStatics.GetPlayerCharacter` 0))))
  (if (== _team WinnerTeam)
    (bind _gm (message `/Game/FPS/Blueprints/Interfaces/BI_GameState.GetGameMode` (`GameplayStatics.GetGameState`)))
    (`self.GameWon` _gm)))

(event `LoadMissions`
  (bind _slot_name (`self.Slot Name`))
  ;[0 0.02868 0.15] Save & Load
  ;;[0 0 0 0.5] Load Missions
  (bind _returnvalue (`GameplayStatics.DoesSaveGameExist` _slot_name))
  (if _returnvalue
    (bind _returnvalue_2 (`GameplayStatics.LoadGameFromSlot` _slot_name))
    (bind _asbp_fps_save_missions (cast `/Game/FPS/Blueprints/SaveGame/BP_FPS_Save_Missions` _returnvalue_2))
    (bind _missions (`/Game/FPS/Blueprints/SaveGame/BP_FPS_Save_Missions.Missions` _asbp_fps_save_missions))
    (if (`KismetArrayLibrary.Array_IsValidIndex` _missions)
      (set `self.Missions` _missions)
      (`self.SaveProgress`))
    (else
      (`self.Create DefaultMissions`))))

(event `SaveProgress`
  ;[0 0.02868 0.15] Save & Load
  ;;[0 0 0] Save Mission Progress
  (bind _returnvalue (`GameplayStatics.CreateSaveGameObject` "/Game/FPS/Blueprints/SaveGame/BP_FPS_Save_Missions.BP_FPS_Save_Missions_C"))
  (set `/Game/FPS/Blueprints/SaveGame/BP_FPS_Save_Missions.Missions` (`self.Missions`) _returnvalue)
  (`AsyncActionHandleSaveGame.AsyncSaveGameToSlot` _returnvalue (`self.Slot Name`)))

(event `Create DefaultMissions`
  ;[0 0.02868 0.15] Save & Load
  ;;[0 0 0 0.5] Default Missions
  (set `self.Missions` (`|MakeArray` (make `/Game/FPS/Blueprints/Data/S_Mission` "/Game/FPS/Blueprints/DataAssets/Mission/DA_Mission_4.DA_Mission_4") (make `/Game/FPS/Blueprints/Data/S_Mission` "/Game/FPS/Blueprints/DataAssets/Mission/DA_Mission_2.DA_Mission_2") (make `/Game/FPS/Blueprints/Data/S_Mission` "/Game/FPS/Blueprints/DataAssets/Mission/DA_Mission_3.DA_Mission_3")))
  (`self.SaveProgress`))

(event `PlayerKilled`
  (params (WeaponType :type "/Game/FPS/Blueprints/Enums/E_WeaponType Enum" :default "NewEnumerator0"))
  ;[0 0 0 0.5] PlayerKilled
  (`self.CheckMissionsPlayersKilled` WeaponType))

(event `GameWon`
  (params (GameMode :type "/Game/FPS/Maps/Enums/EGameModes Enum" :default "NewEnumerator4"))
  ;[0 0 0 0.5] Game Won
  (`self.CheckMissionsGamesWon` GameMode))

(fn `CheckMissionsGamesWon`
  (params (InputPin :type "/Game/FPS/Maps/Enums/EGameModes Enum" :default "NewEnumerator4"))
  (for (_array_element _array_index) (`self.Missions`)
    (bind (_misioninfo _currentprogress) (break `/Game/FPS/Blueprints/Data/S_Mission` _array_element))
    (if (`/Game/FPS/Blueprints/DataAssets/Mission/PDA_Mission.bNeedsWins` _misioninfo)
      (if (`/Game/FPS/Blueprints/DataAssets/Mission/PDA_Mission.bNeedsSpecificGameMode` _misioninfo)
        (if (`|EnumEquality` (`/Game/FPS/Blueprints/DataAssets/Mission/PDA_Mission.GameModeNeeded` _misioninfo) InputPin)
          (bind _structout (setmembers `/Game/FPS/Blueprints/Data/S_Mission` :`StructRef` _array_element :`CurrentProgress` (+ _currentprogress 1) :!label _label))
          (`KismetArrayLibrary.Array_Set` (`self.Missions`) _array_index _structout)
          (`self.SaveProgress`)
          (if (>= _currentprogress (`/Game/FPS/Blueprints/DataAssets/Mission/PDA_Mission.Target` _misioninfo))
            (setmembers `/Game/FPS/Blueprints/Data/S_Mission` :`StructRef` _array_element :`bCompleted` true)
            (`KismetArrayLibrary.Array_Set` (`self.Missions`) _array_index _array_element)
            (message `/Game/FPS/Blueprints/Interfaces/BI_PlayerState.GiveExp` (`self.GetOwner`) (`/Game/FPS/Blueprints/DataAssets/Mission/PDA_Mission.ExpReward` _misioninfo))))
        (else
          (goto _label))))))

(fn `CheckMissionsPlayersKilled`
  (params (WeaponType :type "/Game/FPS/Blueprints/Enums/E_WeaponType Enum" :default "NewEnumerator0"))
  (for (_array_element _array_index) (`self.Missions`)
    (bind (_misioninfo _currentprogress _bcompleted) (break `/Game/FPS/Blueprints/Data/S_Mission` _array_element))
    (if _bcompleted
      _
      (elif (`/Game/FPS/Blueprints/DataAssets/Mission/PDA_Mission.bNeedsKills` _misioninfo)
        (if (`/Game/FPS/Blueprints/DataAssets/Mission/PDA_Mission.bNeedSpecificWeapon` _misioninfo)
          (if (`|EnumEquality` (`/Game/FPS/Blueprints/DataAssets/Mission/PDA_Mission.WeaponNeeded` _misioninfo) WeaponType)
            (bind _structout (setmembers `/Game/FPS/Blueprints/Data/S_Mission` :`StructRef` _array_element :`CurrentProgress` (+ _currentprogress 1) :!label _label))
            (`KismetArrayLibrary.Array_Set` (`self.Missions`) _array_index _structout)
            (if (>= _currentprogress (`/Game/FPS/Blueprints/DataAssets/Mission/PDA_Mission.Target` _misioninfo))
              (bind _structout_2 (setmembers `/Game/FPS/Blueprints/Data/S_Mission` :`StructRef` _array_element :`bCompleted` true))
              (`KismetArrayLibrary.Array_Set` (`self.Missions`) _array_index _structout_2)
              (message `/Game/FPS/Blueprints/Interfaces/BI_PlayerState.GiveExp` (`self.GetOwner`) (`/Game/FPS/Blueprints/DataAssets/Mission/PDA_Mission.ExpReward` _misioninfo)))
            (`self.SaveProgress`))
          (else
            (goto _label)))))))