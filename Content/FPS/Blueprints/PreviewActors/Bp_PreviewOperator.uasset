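; Preview actor that displays the selected loadout operator for its team, posed with a weapon.
; BeginPlay retries until a player controller exists, sets both teams' preview operators through AC_Loadout, and subscribes to operator changes.
; Operator meshes load asynchronously, with the initial looping animation randomized in rate and start position to vary poses.
; Weapon mesh and transform follow WeaponType, while SetAnimation alternates between rifle and machine gun poses.
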(event `self.ReceiveBeginPlay`
  (bind _returnvalue (`GameplayStatics.GetPlayerController` 0))
  (bind _animation (`self.Animation`))
  (bind _skeletalmesh (`self.SkeletalMesh`))
  (`/Engine/EditorBlueprintResources/StandardMacros.IsValid` _returnvalue :!label _label ; ensure that the controller is valid
    (:`Is Valid`
      (bind _output_get (set `self.Controller` _returnvalue))
      (bind _returnvalue_2 (`self.GetComponentByClass` _output_get "/Game/FPS/Blueprints/BlueprintsComponents/AC_Loadout.AC_Loadout_C"))
      (bind _output_get_2 (set `self.LoadoutComponent` _returnvalue_2))
      (`/Game/FPS/Blueprints/BlueprintsComponents/AC_Loadout.SetPreviewOperator` _returnvalue_2 (`/Game/FPS/Blueprints/BlueprintsComponents/AC_Loadout.OperatorClassA` _output_get_2) 0)
      (`/Game/FPS/Blueprints/BlueprintsComponents/AC_Loadout.SetPreviewOperator` _output_get_2 (`/Game/FPS/Blueprints/BlueprintsComponents/AC_Loadout.OperatorClassB` _output_get_2) 1)
      (`self.SetWeapon`)
      (add `/Game/FPS/Blueprints/BlueprintsComponents/AC_Loadout.PreviewOperatorChanged` _returnvalue_2 (delegate `SetPreviewOperator`))
      (bind _returnvalue_3 (select `int` (`self.Team`) :`0` (`/Game/FPS/Blueprints/DataAssets/Operator/PDA_Operator_Info.SkeletalMesh` (`/Game/FPS/Blueprints/BlueprintsComponents/AC_Loadout.PreviewOperatorMeshA` _output_get_2)) :`1` (`/Game/FPS/Blueprints/DataAssets/Operator/PDA_Operator_Info.SkeletalMesh` (`/Game/FPS/Blueprints/BlueprintsComponents/AC_Loadout.PreviewOperatorMeshB` _output_get_2))))
      (`|LoadAsset` _returnvalue_3
        (:`Completed`
          (`SkeletalMeshComponent.SetSkeletalMeshAsset` (`self.SkeletalMesh`) (`|ConvertAsset` _returnvalue_3))
          (`/Engine/EditorBlueprintResources/StandardMacros.IsValid` _animation
            (:`Is Valid`
              (`SkeletalMeshComponent.PlayAnimation` _skeletalmesh _animation true)
              (`SkeletalMeshComponent.SetPlayRate` _skeletalmesh (`KismetMathLibrary.RandomFloatInRange` 0.8 1.0))
              (`SkeletalMeshComponent.SetPosition` _skeletalmesh (`KismetMathLibrary.RandomFloatInRange` 0.0 3.0) true))))))
    (:`Is Not Valid`
      (`KismetSystemLibrary.Delay` 0.1)
      (goto _label))))

(event `SetWeapon`
  (bind _weapontype (`self.WeaponType`))
  (`SkeletalMeshComponent.SetSkeletalMeshAsset` (`self.WeaponMesh`) (select `/Game/FPS/Blueprints/Enums/E_WeaponNames` _weapontype :`NewEnumerator0` "/Game/FPS/Weapons/AssaultRifle/SKM_AssaultRifle.SKM_AssaultRifle" :`NewEnumerator10` "/Game/FPS/Weapons/Rifle/SKM_Mk11.SKM_Mk11" :!type "SkeletalMesh Object Reference"))
  (`SceneComponent.K2_SetRelativeTransform` (`self.WeaponMesh`) (select `/Game/FPS/Blueprints/Enums/E_WeaponNames` _weapontype :`NewEnumerator0` (`KismetMathLibrary.MakeTransform` (-7.165025 2.993517 1.834516) (struct :`Pitch` 7.448762 :`Yaw` 103.60108 :`Roll` 2.725476)) :`NewEnumerator10` (`KismetMathLibrary.MakeTransform` (-6.236122 3.008201 1.059424) (struct :`Pitch` 3.498951 :`Yaw` 105.081982 :`Roll` 4.057512)) :!type "Transform Structure") false false))

(event `SetPreviewOperator`
  (params (Team :type Integer))
  (bind _loadoutcomponent (`self.LoadoutComponent`))
  (bind _returnvalue (select `int` (`self.Team`) :`0` (`/Game/FPS/Blueprints/DataAssets/Operator/PDA_Operator_Info.SkeletalMesh` (`/Game/FPS/Blueprints/BlueprintsComponents/AC_Loadout.PreviewOperatorMeshA` _loadoutcomponent)) :`1` (`/Game/FPS/Blueprints/DataAssets/Operator/PDA_Operator_Info.SkeletalMesh` (`/Game/FPS/Blueprints/BlueprintsComponents/AC_Loadout.PreviewOperatorMeshB` _loadoutcomponent))))
  (if (== Team (`self.Team`))
    (`|LoadAsset` _returnvalue
      (:`Completed`
        (`SkeletalMeshComponent.SetSkeletalMeshAsset` (`self.SkeletalMesh`) (`|ConvertAsset` _returnvalue))))))

(event `SetAnimation`
  (`/Engine/EditorBlueprintResources/StandardMacros.FlipFlop`
    (:`A`
      (`SkeletalMeshComponent.SetAnimation` (`self.SkeletalMesh`) "/Game/FPS/Animations/TPP/MenuPoses/A_TPP_AR_Menu_Pose_01.A_TPP_AR_Menu_Pose_01")
      (`SkeletalMeshComponent.SetSkeletalMeshAsset` (`self.WeaponMesh`) "/Game/FPS/Weapons/AssaultRifle/SKM_AssaultRifle.SKM_AssaultRifle")
      (`SceneComponent.K2_SetRelativeTransform` (`self.WeaponMesh`) (`KismetMathLibrary.MakeTransform` (-7.165025 2.993517 1.834516) (struct :`Pitch` 7.448762 :`Yaw` 103.60108 :`Roll` 2.725476)) false false))
    (:`B`
      (`SkeletalMeshComponent.SetAnimation` (`self.SkeletalMesh`) "/Game/FPS/Animations/TPP/MenuPoses/A_TPP_MG_Menu_Pose_04.A_TPP_MG_Menu_Pose_04")
      (`SkeletalMeshComponent.SetSkeletalMeshAsset` (`self.WeaponMesh`) "/Game/FPS/Weapons/MachineGun/SKM_MachineGun_03.SKM_MachineGun_03")
      (`SceneComponent.K2_SetRelativeTransform` (`self.WeaponMesh`) (`KismetMathLibrary.MakeTransform` (-7.165025 2.993517 1.834516) (struct :`Pitch` 7.448762 :`Yaw` 103.60108 :`Roll` 2.725476)) false false))))

(fn `UserConstructionScript`
  (`SceneComponent.K2_SetRelativeRotation` (`self.SkeletalMesh`) (`KismetMathLibrary.MakeRotator` 0.0 0.0 (`self.New Rotation Z (Yaw)`)) false false))