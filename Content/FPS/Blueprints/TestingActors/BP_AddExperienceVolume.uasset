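; BP_AddExperienceVolume is a testing actor that grants a configurable amount of experience to pawns entering its box.
; On box overlap, it casts the other actor to Pawn and calls AddExperience on the AC_PlayerStateInfo component of that pawn's PlayerState.
; The construction script writes the amount into a text render label as "{x} exp".
; Every new overlap grants experience again, with no cooldown or authority check.
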(event `self.Box.OnComponentBeginOverlap`
  (params (OverlappedComponent :type "PrimitiveComponent Object Reference") (OtherActor :type "Actor Object Reference") (OtherComp :type "PrimitiveComponent Object Reference") (OtherBodyIndex :type Integer) (bFromSweep :type Boolean) (SweepResult :type "HitResult Structure (by ref)"))
  (bind _aspawn (cast `Pawn` OtherActor))
  (`/Game/FPS/Blueprints/BlueprintsComponents/AC_PlayerStateInfo.AddExperience` (`self.GetComponentByClass` (`Pawn.PlayerState` _aspawn) "/Game/FPS/Blueprints/BlueprintsComponents/AC_PlayerStateInfo.AC_PlayerStateInfo_C") (`self.Experience to Add`)))

(fn `UserConstructionScript`
  (`TextRenderComponent.K2_SetText` (`self.TextRender`) (`|FormatText` "{x} exp" (`KismetTextLibrary.Conv_IntToText` (`self.Experience to Add`)))))